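; Fire hazard Blueprint that damages the player while a third-person character is inside its sphere trigger.
; Sphere begin and end overlaps with BP_ThirdPersonCharacter toggle the FireDamageOn flag and print its value.
; Tick runs through a short Delay to throttle damage, then applies a fixed amount to player character 0 while the flag is set.
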(event OnComponentBeginOverlap(Sphere)
  (params (OverlappedComponent :type Primitive%20Component%20Object%20Reference) (OtherActor :type Actor%20Object%20Reference) (OtherComp :type Primitive%20Component%20Object%20Reference) (OtherBodyIndex :type Integer) (bFromSweep :type Boolean) (SweepResult :type Hit%20Result%20Structure%20%28by%20ref%29))
  (Utilities|Casting|CastToBP_ThirdPersonCharacter OtherActor)
  (bind _output_get (Variables|Default|SetFireDamageOn true))
  (Development|PrintString (Utilities|String|ToString(Boolean) _output_get)))

(event OnComponentEndOverlap(Sphere)
  (params (OverlappedComponent :type Primitive%20Component%20Object%20Reference) (OtherActor :type Actor%20Object%20Reference) (OtherComp :type Primitive%20Component%20Object%20Reference) (OtherBodyIndex :type Integer))
  (Utilities|Casting|CastToBP_ThirdPersonCharacter OtherActor)
  (bind _output_get (Variables|Default|SetFireDamageOn false))
  (Development|PrintString (Utilities|String|ToString(Boolean) _output_get)))

(event EventTick
  (params (DeltaSeconds :type Float%20%28single-precision%29))
  (Utilities|FlowControl|Delay 0.1)
  (if (Variables|Default|GetFireDamageOn)
    (Game|Damage|ApplyDamage (Game|GetPlayerCharacter 0) 1e+01 0 0)))

(fn ConstructionScript)